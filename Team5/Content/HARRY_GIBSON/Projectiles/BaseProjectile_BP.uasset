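; Base projectile actor that damages BaseEnemy actors on overlap.
; On BeginPlay it either tints its mesh through colour and emissive material parameters (SimpleProjectile) or swaps in a custom static mesh at unit scale.
; The first enemy overlap, gated by DoOnce, sends a health message with triple damage if the projectile overlaps the enemy's CriticalHitBox, then spawns sparks at the enemy and destroys itself.
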(event `self.ReceiveBeginPlay`
  (bind _projectile (`self.Projectile`))
  (bind _projectile_2 (`self.Projectile`))
  ;[1 1 1] Set Initial Variables
  (if (`self.SimpleProjectile?`)
    (`MeshComponent.SetVectorParameterValueOnMaterials` _projectile (`self.ProjectileColour`) (`self.ColourValue`))
    (`MeshComponent.SetScalarParameterValueOnMaterials` _projectile (`self.EmissiveIntensity`) (`self.EmissiveIntensityValue`))
    (else
      (`StaticMeshComponent.SetStaticMesh` _projectile_2 (`self.ProjectileMesh`))
      (`SceneComponent.SetWorldScale3D` _projectile_2 (1.0 1.0 1.0)))))

(event `self.ProjectileCollision.OnComponentBeginOverlap`
  (params (OverlappedComponent :type "PrimitiveComponent Object Reference") (OtherActor :type "Actor Object Reference") (OtherComp :type "PrimitiveComponent Object Reference") (OtherBodyIndex :type Integer) (bFromSweep :type Boolean) (SweepResult :type "HitResult Structure (by ref)"))
  (bind _projectiledamage (`self.ProjectileDamage`))
  ;[1 1 1] Damage
  (bind _asbase_enemy (cast `/Game/HARRY_GIBSON/BaseEnemy` OtherActor))
  (`/Engine/EditorBlueprintResources/StandardMacros.DoOnce` false
    (:`Completed`
      (if (`PrimitiveComponent.IsOverlappingActor` (`/Game/HARRY_GIBSON/BaseEnemy.Critical Hit Box` _asbase_enemy) self)
        (message `/Game/HARRY_GIBSON/iDamageable.AffectHealth` _asbase_enemy (* _projectiledamage 3.0))
        (else
          (message `/Game/HARRY_GIBSON/iDamageable.AffectHealth` _asbase_enemy _projectiledamage)))
      (`GameplayStatics.SpawnEmitterAtLocation` "/Game/HARRY_GIBSON/P_Sparks.P_Sparks" (`self.K2_GetActorLocation` _asbase_enemy))
      (`self.K2_DestroyActor`))))

(fn `UserConstructionScript`)